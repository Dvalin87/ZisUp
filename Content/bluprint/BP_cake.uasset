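; BP_cake is a cake actor that lets the player's BP_ThirdPersonCharacter eat while it is within range.
; Its Box overlap events set the character's CanEat flag on entry and clear it on exit.
; The EatMe component starts inactive; Tick polls the player's BiscuitTrigger flag, activates EatMe while it is set, and deactivates it after a one-second delay.
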(event `self.ReceiveBeginPlay`
  (`ActorComponent.Deactivate` (`self.eatMe`)))

(event `self.ReceiveTick`
  (params (DeltaSeconds :type "Float (single-precision)"))
  (bind _eatme (`self.eatMe`))
  (bind _asbp_third_person_character (cast `/Game/ThirdPerson/Blueprints/BP_ThirdPersonCharacter` (`GameplayStatics.GetPlayerCharacter` 0)))
  (if (`/Game/ThirdPerson/Blueprints/BP_ThirdPersonCharacter.biscuitTrigger` _asbp_third_person_character)
    (`ActorComponent.Activate` _eatme false)
    (`KismetSystemLibrary.Delay` 1.0)
    (`ActorComponent.Deactivate` _eatme)))

(event `self.Box.OnComponentBeginOverlap`
  (params (OverlappedComponent :type "PrimitiveComponent Object Reference") (OtherActor :type "Actor Object Reference") (OtherComp :type "PrimitiveComponent Object Reference") (OtherBodyIndex :type Integer) (bFromSweep :type Boolean) (SweepResult :type "HitResult Structure (by ref)"))
  (bind _asbp_third_person_character (cast `/Game/ThirdPerson/Blueprints/BP_ThirdPersonCharacter` OtherActor))
  (set `/Game/ThirdPerson/Blueprints/BP_ThirdPersonCharacter.canEat` true _asbp_third_person_character))

(event `self.Box.OnComponentEndOverlap`
  (params (OverlappedComponent :type "PrimitiveComponent Object Reference") (OtherActor :type "Actor Object Reference") (OtherComp :type "PrimitiveComponent Object Reference") (OtherBodyIndex :type Integer))
  (bind _asbp_third_person_character (cast `/Game/ThirdPerson/Blueprints/BP_ThirdPersonCharacter` OtherActor))
  (set `/Game/ThirdPerson/Blueprints/BP_ThirdPersonCharacter.canEat` false _asbp_third_person_character))

(fn `UserConstructionScript`)